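; Base weapon actor that spins around the vertical axis at a rate tied to the player's current attack value.
; On BeginPlay it caches the first player's BP_TopDownController.
; Each Tick it accumulates elapsed time, reads the current attack from the controller, and sets absolute yaw to time × (attack + 1) × Speed.
; Yaw is recomputed from total time, so a change in attack makes the angle jump.
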(event `self.ReceiveBeginPlay`
  (bind _asbp_top_down_controller (cast `/Game/TopDown/Blueprints/BP_TopDownController` (`GameplayStatics.GetPlayerController` 0)))
  (set `self.Controller` _asbp_top_down_controller))

(event `self.ReceiveTick`
  (params (DeltaSeconds :type "Float (single-precision)"))
  (bind _output_get (set `self.totaltime` (+ DeltaSeconds (`self.totaltime`))))
  (bind _currentattack (`/Game/TopDown/Blueprints/BP_TopDownController.GetCurrentAttack` (`self.Controller`)))
  (`self.K2_SetActorRotation` (`KismetMathLibrary.MakeRotator` 0.0 0.0 (* _output_get (* (+ _currentattack 1) (`self.speed`))))))

(fn `UserConstructionScript`)