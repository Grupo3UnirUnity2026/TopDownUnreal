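; Boomerang weapon actor that flies out along a forward vector and returns to the player.
; BeginPlay caches start position, owner's facing and the top-down controller.
; Tick moves it to ThrowDistance, then homes toward PlayerRef, snapping to HammerSpawnPoint when close and restarting outward.
; UpgradeAttack runs every tick, reading current attack but setting MoveSpeed to zero, which halts that movement; PlayerRef is never assigned here.
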(event `self.ReceiveBeginPlay`
  (bind _asbp_garret_simple (cast `/Game/Polyart/ModularStylizedChars/Blueprints/Actors/Characters/BP_GarretSimple` (`self.GetOwner`)))
  (bind _output_get (set `self.StartLocation` (`self.K2_GetActorLocation`)))
  (bind _output_get_2 (set `self.ForwardVector` (`self.GetActorForwardVector` _asbp_garret_simple)))
  (set `self.EndLocation` (* (+ _output_get _output_get_2) (`self.ThrowDistance`)))
  (bind _asbp_top_down_controller (cast `/Game/TopDown/Blueprints/BP_TopDownController` (`GameplayStatics.GetPlayerController` 0)))
  (set `self.PlayerController` _asbp_top_down_controller))

(event `self.ReceiveTick`
  (params (DeltaSeconds :type "Float (single-precision)"))
  (`/Engine/EditorBlueprintResources/StandardMacros.IsValid` (`self.PlayerRef`)
    (:`Is Valid`
      (`self.UpgradeAttack`)
      (if (`self.IsReturning`)
        (`self.K2_SetActorLocation` (+ (`self.K2_GetActorLocation`) (* (* (`KismetMathLibrary.Vector_Normal2D` (- (`self.K2_GetActorLocation` (`self.PlayerRef`)) (`self.K2_GetActorLocation`))) (`self.MoveSpeed`)) DeltaSeconds)))
        (if (<= (`KismetMathLibrary.Vector_Distance` (`self.K2_GetActorLocation`) (`self.K2_GetActorLocation` (`self.PlayerRef`))) 200.0)
          (`self.K2_SetActorLocation` (`SceneComponent.K2_GetComponentLocation` (`/Game/Polyart/ModularStylizedChars/Blueprints/Actors/Characters/BP_GarretSimple.HammerSpawnPoint` (`self.PlayerRef`))))
          (set `self.IsReturning` false)
          (set `self.StartLocation` (`self.K2_GetActorLocation`))
          (set `self.ForwardVector` (`self.GetActorForwardVector` (`self.PlayerRef`))))
        (else
          (`self.K2_SetActorLocation` (+ (* DeltaSeconds (* (`self.MoveSpeed`) (`self.ForwardVector`))) (`self.K2_GetActorLocation`)))
          (if (>= (`KismetMathLibrary.Vector_Distance` (`self.StartLocation`) (`self.K2_GetActorLocation`)) (`self.ThrowDistance`))
            (set `self.IsReturning` true)))))))

(event `UpgradeAttack`
  (bind _currentattack (`/Game/TopDown/Blueprints/BP_TopDownController.GetCurrentAttack` (`self.PlayerController`)))
  (set `self.MoveSpeed` 0.0))

(fn `UserConstructionScript`)