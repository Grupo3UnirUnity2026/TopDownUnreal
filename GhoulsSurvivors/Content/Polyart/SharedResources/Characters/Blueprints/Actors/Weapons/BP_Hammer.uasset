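; Hammer weapon actor that slams down, damaging BP_TestingWeapons actors in its impact sphere.
; On BeginPlay, a Timeline lowers it from above its spawn height and drives pitch, while X, Y and yaw track the HammerSpawnPoint of its BP_GarretSimple owner.
; When the swing finishes, it spawns impact VFX, camera shake and sound, applies damage through ReceiveDamage, then destroys itself after LifeTime.
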(event `self.ReceiveBeginPlay`
  (bind (_updaterotation_roll _updaterotation_pitch _updaterotation_yaw) (`KismetMathLibrary.BreakRotator` (`self.UpdateRotation`)))
  (bind (_updateposition_x _updateposition_y) (`KismetMathLibrary.BreakVector` (`self.UpdatePosition`)))
  (set `self.InitialRotation` (`self.K2_GetActorRotation`))
  (bind _output_get (set `self.EndLocation` (`self.K2_GetActorLocation`)))
  (bind _output_get_2 (set `self.Startlocation` (+ _output_get (0.0 0.0 200.0))))
  (bind (_direction _alpha _rotation) (`Timeline|Timeline`)
    (:`Update`
      (`self.PlayerRotator`)
      (`self.PlayerMovement`)
      (bind (_returnvalue_x _returnvalue_y _returnvalue_z) (`KismetMathLibrary.BreakVector` (`KismetMathLibrary.VLerp` _output_get_2 _output_get _alpha)))
      (`self.K2_SetActorLocation` (`KismetMathLibrary.MakeVector` _updateposition_x _updateposition_y _returnvalue_z))
      (`self.K2_SetActorRotation` (`KismetMathLibrary.MakeRotator` 0.0 _rotation _updaterotation_yaw)))
    (:`Finished`
      (`NiagaraFunctionLibrary.SpawnSystemAtLocation` (`self.HammerImpact`) (`self.K2_GetActorLocation`))
      (`GameplayStatics.PlayWorldCameraShake` "/Game/Polyart/SharedResources/Characters/Blueprints/Actors/Weapons/CS_HammerImpact.CS_HammerImpact_C" (`self.K2_GetActorLocation`) 1000.0 2000.0)
      (`self.HammerAttack`)
      (`GameplayStatics.PlaySound2D` null 1.0 1.0 0.0 null null)
      (`KismetSystemLibrary.Delay` (`self.LifeTime`))
      (`self.K2_DestroyActor`))))

(event `self.ReceiveTick`
  (params (DeltaSeconds :type "Float (single-precision)")))

(event `HammerAttack`
  ; Attack
  (for _array_element (`PrimitiveComponent.GetOverlappingActors` (`self.Sphere`) "/Game/Polyart/SharedResources/Characters/Blueprints/Actors/Weapons/BP_TestingWeapons.BP_TestingWeapons_C")
    (bind _asbp_testing_weapons (cast `/Game/Polyart/SharedResources/Characters/Blueprints/Actors/Weapons/BP_TestingWeapons` _array_element))
    (`/Game/Polyart/SharedResources/Characters/Blueprints/Actors/Weapons/BP_TestingWeapons.ReceiveDamage` _asbp_testing_weapons (`self.Damage`))
    (`KismetSystemLibrary.PrintString` "Hit")))

(event `PlayerRotator`
  (bind _asbp_garret_simple (cast `/Game/Polyart/ModularStylizedChars/Blueprints/Actors/Characters/BP_GarretSimple` (`self.GetOwner`)))
  (set `self.UpdateRotation` (`SceneComponent.K2_GetComponentRotation` (`/Game/Polyart/ModularStylizedChars/Blueprints/Actors/Characters/BP_GarretSimple.HammerSpawnPoint` _asbp_garret_simple))))

(event `PlayerMovement`
  (bind _asbp_garret_simple (cast `/Game/Polyart/ModularStylizedChars/Blueprints/Actors/Characters/BP_GarretSimple` (`self.GetOwner`)))
  (set `self.UpdatePosition` (`SceneComponent.K2_GetComponentLocation` (`/Game/Polyart/ModularStylizedChars/Blueprints/Actors/Characters/BP_GarretSimple.HammerSpawnPoint` _asbp_garret_simple))))

(fn `UserConstructionScript`)