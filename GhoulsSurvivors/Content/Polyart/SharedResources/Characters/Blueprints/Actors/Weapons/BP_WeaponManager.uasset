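; Weapon manager actor that spawns and swaps the player's equipped weapons, a sword or a hammer.
; StartWeaponManager activates each equipped entry: the sword spawns once, while the hammer respawns on a looping cooldown timer, both at player spawn points and owned by the player.
; AddWeapon replaces the loadout with a new weapon type, destroying every actor tagged "Weapon" but leaving any hammer timer running.
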(event `self.ReceiveTick`
  (params (DeltaSeconds :type "Float (single-precision)")))

(fn `ActivateWeapon`
  (params (WeaponType :type "/Game/Polyart/SharedResources/Characters/Blueprints/Actors/Weapons/E_WeaponType Enum" :default "NewEnumerator0"))
  (switch `/Game/Polyart/SharedResources/Characters/Blueprints/Actors/Weapons/E_WeaponType` WeaponType
    (:`NewEnumerator0`
      (`self.Start Hammer`))
    (:`NewEnumerator1`
      (`self.SpawnSword`))))

(fn `AddWeapon `
  (params (NewWeapon :type "/Game/Polyart/SharedResources/Characters/Blueprints/Actors/Weapons/E_WeaponType Enum" :default "NewEnumerator0"))
  (if (not (`KismetArrayLibrary.Array_Contains` (`self.EquipedWeapon`) (`local.NewWeapon`)))
    (`self.ClearCurrentWeapon`)
    (`KismetArrayLibrary.Array_Clear` (`self.EquipedWeapon`))
    (`KismetArrayLibrary.Array_Add` (`self.EquipedWeapon`) (`local.NewWeapon`))
    (`self.ActivateWeapon` (`local.NewWeapon`))))

(fn `ClearCurrentWeapon`
  (bind _outactors (`GameplayStatics.GetAllActorsWithTag` "Weapon"))
  (for _array_element _outactors
    (`self.K2_DestroyActor` _array_element)))

(fn `SpawnHammer`
  (bind _returnvalue (`|SpawnActorFromClass` (`self.HammerClass`) (`SceneComponent.K2_GetComponentToWorld` (`/Game/Polyart/ModularStylizedChars/Blueprints/Actors/Characters/BP_GarretSimple.HammerSpawnPoint` (`self.PlayerReference`))) "Undefined" "MultiplyWithRoot" null null))
  (`self.SetOwner` _returnvalue (`self.PlayerReference`)))

(fn `SpawnSword`
  (bind _returnvalue (`|SpawnActorFromClass` "/Game/Polyart/SharedResources/Characters/Blueprints/Actors/Weapons/BP_WeaponBase.BP_WeaponBase_C" (`SceneComponent.K2_GetComponentToWorld` (`/Game/Polyart/ModularStylizedChars/Blueprints/Actors/Characters/BP_GarretSimple.SwordSpawnPoint` (`self.PlayerReference`))) "Undefined" "MultiplyWithRoot" null null))
  (`self.SetOwner` _returnvalue (`self.PlayerReference`)))

(fn `Start Hammer`
  (`KismetSystemLibrary.K2_SetTimer` null "SpawnHammer" (`self.HammerCooldown`) true))

(fn `StartWeaponManager`
  (for _array_element (`self.EquipedWeapon`)
    (`self.ActivateWeapon` _array_element)))

(fn `UserConstructionScript`)