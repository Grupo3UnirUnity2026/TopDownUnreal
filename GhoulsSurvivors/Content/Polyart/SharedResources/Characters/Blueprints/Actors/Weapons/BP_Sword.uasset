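; BP_Sword is a sword weapon actor that circles a center point at a fixed height offset.
; Each Tick it advances an angle by orbit speed scaled by delta time, converts it with cosine and sine, and scales by the orbit radius.
; The result sets the actor's relative location without sweep, so the orbit follows any parent it is attached to.
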(event `self.ReceiveBeginPlay`)

(event `self.ReceiveTick`
  (params (DeltaSeconds :type "Float (single-precision)"))
  (bind _output_get (set `self.CurrentAngle` (+ (* (`self.OrbitSpeed`) DeltaSeconds) (`self.CurrentAngle`))))
  (bind _returnvalue (`KismetMathLibrary.DegreesToRadians` _output_get))
  (`self.K2_SetActorRelativeLocation` (`KismetMathLibrary.MakeVector` (* (`KismetMathLibrary.Cos` _returnvalue) (`self.OrbitRadius`)) (* (`KismetMathLibrary.Sin` _returnvalue) (`self.OrbitRadius`)) (`self.HeighOffset`))))

(fn `UserConstructionScript`)