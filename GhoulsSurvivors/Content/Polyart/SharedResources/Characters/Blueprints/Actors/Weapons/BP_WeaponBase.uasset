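; BP_WeaponBase is a base weapon actor that orbits or spins at the sword spawn point of its owning BP_GarretSimple character.
; BeginPlay caches the first player's BP_TopDownController, which supplies the current attack value.
; Each Tick teleport-free moves the actor to the owner's SwordSpawnPoint without sweeping.
; Its yaw comes from accumulated time multiplied by that attack value and Speed, so the attack value scales the spin.
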(event `self.ReceiveBeginPlay`
  (bind _asbp_top_down_controller (cast `/Game/TopDown/Blueprints/BP_TopDownController` (`GameplayStatics.GetPlayerController` 0)))
  (set `self.Controller` _asbp_top_down_controller))

(event `self.ReceiveTick`
  (params (DeltaSeconds :type "Float (single-precision)"))
  (`self.PlayerUpdateMovement`)
  (bind _output_get (set `self.totaltime` (+ DeltaSeconds (`self.totaltime`))))
  (bind _currentattack (`/Game/TopDown/Blueprints/BP_TopDownController.GetCurrentAttack` (`self.Controller`)))
  (`self.K2_SetActorRotation` (`KismetMathLibrary.MakeRotator` 0.0 0.0 (* _output_get (* _currentattack (`self.speed`)))))
  (`self.K2_SetActorLocation` (`self.UpdatePosition`)))

(event `PlayerUpdateMovement`
  (bind _asbp_garret_simple (cast `/Game/Polyart/ModularStylizedChars/Blueprints/Actors/Characters/BP_GarretSimple` (`self.GetOwner`)))
  (set `self.UpdatePosition` (`SceneComponent.K2_GetComponentLocation` (`/Game/Polyart/ModularStylizedChars/Blueprints/Actors/Characters/BP_GarretSimple.SwordSpawnPoint` _asbp_garret_simple))))

(fn `UserConstructionScript`)